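; Pollution hazard actor that expands over time and flags the player as taking damage while inside it.
; Box overlap begin and end toggle TakingDamage on the FirstPersonCharacter, with a cough sound played on entry.
; From BeginPlay, the self-calling Size event enlarges the actor's scale every few seconds, slightly more horizontally than vertically, until TimesGrown passes MaxTimesGrown.
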(event `self.ReceiveBeginPlay`
  (`self.Size`))

(event `self.Box.OnComponentEndOverlap`
  (params (OverlappedComponent :type "PrimitiveComponent Object Reference") (OtherActor :type "Actor Object Reference") (OtherComp :type "PrimitiveComponent Object Reference") (OtherBodyIndex :type Integer))
  (bind _asfirst_person_character (cast `/Game/FirstPersonBP/Blueprints/FirstPersonCharacter` OtherActor))
  (set `/Game/FirstPersonBP/Blueprints/FirstPersonCharacter.TakingDamage` false _asfirst_person_character))

(event `self.Box.OnComponentBeginOverlap`
  (params (OverlappedComponent :type "PrimitiveComponent Object Reference") (OtherActor :type "Actor Object Reference") (OtherComp :type "PrimitiveComponent Object Reference") (OtherBodyIndex :type Integer) (bFromSweep :type Boolean) (SweepResult :type "HitResult Structure (by ref)"))
  (bind _asfirst_person_character (cast `/Game/FirstPersonBP/Blueprints/FirstPersonCharacter` OtherActor))
  (set `/Game/FirstPersonBP/Blueprints/FirstPersonCharacter.TakingDamage` true _asfirst_person_character)
  (`GameplayStatics.PlaySound2D` "/Game/Sounds/cough.cough" 1.0 1.0 0.0 null null))

(event `Size`
  (if (<= (`self.TimesGrown`) (`self.MaxTimesGrown`))
    (`KismetSystemLibrary.Delay` 3.0)
    (bind _output_get (set `self.NewSize` (+ (`self.NewSize`) (1.25 1.25 1.0))))
    (`self.SetActorScale3D` _output_get)
    (`self.Size`)
    (`/Engine/EditorBlueprintResources/StandardMacros.IncrementInt` (`self.TimesGrown`))))

(fn `UserConstructionScript`)